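; BP_Socket is a puzzle socket that reacts when a BP_PuzzleKey of the required cube type overlaps its Box.
; A match updates its state and cylinder material, sets the intensity of the DirectionalLight found at BeginPlay, and eases the first "Tagged" static mesh actor to a hardcoded transform.
; A wrong type sets another state, and both failure cases print red messages.
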(event `self.ReceiveBeginPlay`
  (bind _returnvalue (`GameplayStatics.GetActorOfClass` "/Script/Engine.DirectionalLight"))
  (set `self.LightSource` _returnvalue))

(event `self.Box.OnComponentBeginOverlap`
  (params (OverlappedComponent :type "PrimitiveComponent Object Reference") (OtherActor :type "Actor Object Reference") (OtherComp :type "PrimitiveComponent Object Reference") (OtherBodyIndex :type Integer) (bFromSweep :type Boolean) (SweepResult :type "HitResult Structure (by ref)"))
  (bind _asbp_puzzle_key (cast `/Game/MyFolder/Blueprints/BP_PuzzleKey` OtherActor)
    (:`then`
      (if (`|EnumEquality` (`/Game/MyFolder/Blueprints/BP_PuzzleKey.CubeType` _asbp_puzzle_key) "NewEnumerator1")
        (`KismetSystemLibrary.PrintString` (`self.SuccessMessage`) true true (struct :`G` 1.0 :`B` 0.139199 :`A` 1.0))
        (set `self.CurrentState` "NewEnumerator3")
        (`PrimitiveComponent.SetMaterial` (`self.Cylinder`) 0 "/Game/MyFolder/Materials/M_MyMaterial_TriggerActive.M_MyMaterial_TriggerActive")
        (`LightComponent.SetIntensity` (`Light.LightComponent` (`self.LightSource`)) 0.3)
        (bind _outactors (`GameplayStatics.GetAllActorsWithTag` "Tagged"))
        (bind _asstatic_mesh_actor (cast `StaticMeshActor` (`|GetArrayItem` _outactors)))
        (`KismetSystemLibrary.MoveComponentTo` (`Actor.RootComponent` _asstatic_mesh_actor) (2795.0 -1554.0 1837.0) (struct :`Pitch` 360.0 :`Yaw` 90.0 :`Roll` -540.0) true false 5.0)
        (else
          (`KismetSystemLibrary.PrintString` (`self.ErrorMessage`) true true (struct :`R` 1.0 :`B` 0.010546 :`A` 1.0))
          (set `self.CurrentState` "NewEnumerator2"))))
    (:`CastFailed`
      (`KismetSystemLibrary.PrintString` (`self.CastFailedMessage`) true true (struct :`R` 1.0 :`B` 0.167214 :`A` 1.0)))))

(fn `UserConstructionScript`)