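; BP_PuzzleGameMode is a puzzle game mode that tracks three puzzle elements and announces a win when all are active.
; UpdatePuzzleState maps an element ID to one of three solved flags, sets or clears it, then runs CheckWinCondition.
; When all three flags are true, that check prints the win message and plays a particle effect and confirm sound at fixed world locations.
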(event `UpdatePuzzleState`
  (params (ElementId :type Integer) (IsActivated :type Boolean))
  (switch `int` ElementId
    (:`0`
      (set `self.IsElement1Solved` IsActivated)
      (`self.CheckWinCondition`))
    (:`1`
      (set `self.IsElement2Solved` IsActivated)
      (`self.CheckWinCondition`))
    (:`2`
      (set `self.IsElement3Solved` IsActivated)
      (`self.CheckWinCondition`))))

(event `CheckWinCondition`
  (if (and (`self.IsElement1Solved`) (`self.IsElement2Solved`) (`self.IsElement3Solved`))
    (`KismetSystemLibrary.PrintString` (`self.WinMessage`) true true (struct :`G` 1.0 :`B` 0.245672 :`A` 1.0) 5.0)
    (`GameplayStatics.SpawnEmitterAtLocation` "/Engine/Functions/Engine_MaterialFunctions02/ExampleContent/3dParticleOpacity_Particle.3dParticleOpacity_Particle" (1.0 2.0 1.0))
    (`GameplayStatics.PlaySoundAtLocation` "/Engine/VREditor/Sounds/VR_confirm_Cue.VR_confirm_Cue" (0.0 0.0 0.0) (struct) 1.0 1.0 0.0 null null null null)))

(fn `UserConstructionScript`)